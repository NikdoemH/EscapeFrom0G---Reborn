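; BP_Drawer is an interactable drawer that opens when the player has a key and spawns a key card as its content.
; BeginInteraction casts the player to BP_FirstPersonCharacter and checks HasKey before playing the Drawer timeline.
; Each timeline update moves the Cube's relative location, then runs into a Delay that leads to spawning BP_KeyCard at a hardcoded location.
; The spawn hangs off Update rather than Finished, with no explicit once-only guard.
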(event EventBeginInteraction
  ;[1 1 1] Casting to BP_FirstPersonCharacter
  (bind _asbp_first_person_character (Utilities|Casting|CastToBP_FirstPersonCharacter (Game|GetPlayerCharacter 0)))
  ;[1 1 1] Checking if player has the key to drawer
  (if (Variables|/Game/FirstPerson/Blueprints/BP_FirstPersonCharacter.BP_FirstPersonCharacter_C|GetHasKey? _asbp_first_person_character)
    ;[1 1 1] Opening drawer
    (bind _opendrawer (Timeline|Drawer Play)
      (:Update
        (Transformation|SetRelativeLocation (Variables|Default|GetCube) _opendrawer false false)
        ;[1 1 1] Spawning content of the drawer
        (Utilities|FlowControl|Delay 1.0)
        (Game|SpawnActorfromClass "/Game/Blueprints/BP_KeyCard.BP_KeyCard_C" (Math|Transform|MakeTransform "-630.000000,-3320.000000,86.000000" "0, 0, 0" "1.000000,1.000000,1.000000") "Undefined" 0 0)))))

(fn ConstructionScript
  (|CallParentFunction))
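; Right-side escape pod door Blueprint that opens when something overlaps its trigger Box after the lever is pulled.
; On overlap it takes the first BP_Lever found in the level and checks IsLeverPulled.
; The OpenRightDoor timeline moves the door's relative location; its Update pin also starts a two-second Delay.
; The CloseRightDoor timeline then plays in reverse from the end to close the door.
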(event OnComponentBeginOverlap(Box)
  (params (OverlappedComponent :type Primitive%20Component%20Object%20Reference) (OtherActor :type Actor%20Object%20Reference) (OtherComp :type Primitive%20Component%20Object%20Reference) (OtherBodyIndex :type Integer) (bFromSweep :type Boolean) (SweepResult :type Hit%20Result%20Structure%20%28by%20ref%29))
  ;[1 1 1] Casting to BP_Lever
  (bind _outactors (Actor|GetAllActorsOfClass "/Game/Blueprints/BP_Lever.BP_Lever_C"))
  (bind _asbp_lever (Utilities|Casting|CastToBP_Lever (Utilities|Array|Get(acopy) _outactors)))
  ;[1 1 1] Checking if player pulled the lever
  (if (Variables|/Game/Blueprints/BP_Lever.BP_Lever_C|GetIsLeverPulled? _asbp_lever)
    ;[1 1 1] Opening doors
    (bind _open (Timeline|OpenRightDoor PlayFromStart)
      (:Update
        (Transformation|SetRelativeLocation (Variables|Default|GetEscapePodDoor_Right) _open false false)
        (Utilities|FlowControl|Delay 2.0)
        ;[1 1 1] Closing doors
        (bind _close (Timeline|CloseRightDoor ReverseFromEnd)
          (:Update
            (Transformation|SetRelativeLocation (Variables|Default|GetEscapePodDoor_Right) _close false false)))))))

(fn ConstructionScript)
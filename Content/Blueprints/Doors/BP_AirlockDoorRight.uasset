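; BP_AirlockDoorRight is an airlock door that slides open and closed, gated on the player having a spacesuit.
; Actor begin and end overlap check HasSpacesuit on the first-person player character, without checking which actor overlapped.
; The AirlockDoors timeline drives the door component's relative location, playing from start on entry and reversing from end on exit.
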(event Collision|EventActorBeginOverlap
  (params (OtherActor :type Actor%20Object%20Reference))
  ;[1 1 1] Casting to BP_FirstPersonCharacter
  (bind _asbp_first_person_character (Utilities|Casting|CastToBP_FirstPersonCharacter (Game|GetPlayerCharacter 0)))
  ;[1 1 1] Checking if player has a spacesuit
  (if (Variables|/Game/FirstPerson/Blueprints/BP_FirstPersonCharacter.BP_FirstPersonCharacter_C|GetHasSpacesuit? _asbp_first_person_character)
    ;[1 1 1] Opening/Closing doors
    (bind _airlockdoor (Timeline|AirlockDoors PlayFromStart)
      (:Update
        (Transformation|SetRelativeLocation (Variables|Default|GetAirlockDoor) _airlockdoor false false)))))

(event Collision|EventActorEndOverlap
  (params (OtherActor :type Actor%20Object%20Reference))
  ;[1 1 1] Casting to BP_FirstPersonCharacter
  (bind _asbp_first_person_character (Utilities|Casting|CastToBP_FirstPersonCharacter (Game|GetPlayerCharacter 0)))
  ;[1 1 1] Checking if player has a spacesuit
  (if (Variables|/Game/FirstPerson/Blueprints/BP_FirstPersonCharacter.BP_FirstPersonCharacter_C|GetHasSpacesuit? _asbp_first_person_character)
    ;[1 1 1] Opening/Closing doors
    (bind _airlockdoor (Timeline|AirlockDoors ReverseFromEnd)
      (:Update
        (Transformation|SetRelativeLocation (Variables|Default|GetAirlockDoor) _airlockdoor false false)))))

(fn ConstructionScript)
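; BP_DebrisDoor is a door that opens only once its Debris array, the list of removed debris, holds exactly three elements.
; Actor overlap plays a Timeline from the start to slide the Pivot's relative location, and end overlap reverses it from the end under the same check.
; The overlap events do not filter by actor, and this Blueprint only reads the Debris array.
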(event Collision|EventActorBeginOverlap
  (params (OtherActor :type Actor%20Object%20Reference))
  ;[1 1 1] Checking if list of removed debris has 3 elements
  (if (== (Utilities|Array|Length (Variables|Default|GetDebris)) 3)
    ;[1 1 1] Opening/Closing doors
    (bind _newtrack_0 (Timeline|Timeline PlayFromStart)
      (:Update
        (Transformation|SetRelativeLocation (Variables|Default|GetPivot) _newtrack_0 false false)))))

(event Collision|EventActorEndOverlap
  (params (OtherActor :type Actor%20Object%20Reference))
  ;[1 1 1] Checking if list of removed debris has 3 elements
  (if (== (Utilities|Array|Length (Variables|Default|GetDebris)) 3)
    ;[1 1 1] Opening/Closing doors
    (bind _newtrack_0 (Timeline|Timeline ReverseFromEnd)
      (:Update
        (Transformation|SetRelativeLocation (Variables|Default|GetPivot) _newtrack_0 false false)))))

(fn ConstructionScript)
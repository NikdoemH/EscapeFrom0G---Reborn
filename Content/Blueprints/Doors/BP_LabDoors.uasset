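; BP_LabDoors is a lab door that opens when something overlaps its StuckBox, then briefly turns physics on for its Cube.
; The overlap plays a timeline that moves the Pivot, unless IsPhysicsEnabled is already set.
; Chained Delays on the timeline's Update switch Cube physics simulation on, then off again, keeping that flag in step.
; ActorBeginOverlap only calls the parent implementation.
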(event OnComponentBeginOverlap(StuckBox)
  (params (OverlappedComponent :type Primitive%20Component%20Object%20Reference) (OtherActor :type Actor%20Object%20Reference) (OtherComp :type Primitive%20Component%20Object%20Reference) (OtherBodyIndex :type Integer) (bFromSweep :type Boolean) (SweepResult :type Hit%20Result%20Structure%20%28by%20ref%29))
  ;[1 1 1] Checking if physics are enabled
  (if (not (Variables|Default|GetIsPhysicsEnabled?))
    ;[1 1 1] Opening doors
    (bind _newtrack_0 (Timeline|Timeline PlayFromStart)
      (:Update
        (Transformation|SetRelativeLocation (Variables|Default|GetPivot) _newtrack_0 false false)
        (Utilities|FlowControl|Delay 1.8)
        (bind _output_get (Variables|Default|SetIsPhysicsEnabled? true))
        (Physics|SetSimulatePhysics (Variables|Default|GetCube) _output_get)
        (Utilities|FlowControl|Delay 2.0)
        (bind _output_get_2 (Variables|Default|SetIsPhysicsEnabled? false))
        (Physics|SetSimulatePhysics (Variables|Default|GetCube) _output_get_2)))))

(event Collision|EventActorBeginOverlap
  (params (OtherActor :type Actor%20Object%20Reference))
  ;[1 1 1] Normal opening/closing doors
  (|CallParentFunction OtherActor))

(fn ConstructionScript
  (|CallParentFunction))
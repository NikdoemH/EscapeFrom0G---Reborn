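; BP_Debris is an interactable debris piece whose removal counts toward enabling a BP_DebrisDoor.
; On BeginInteraction it finds the first debris door in the level, adds its DebrisID to that door's Debris list and destroys itself.
; When the list holds exactly three entries, it moves the door's collision box to a new relative location, which the author notes the doors need to work.
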(event EventBeginInteraction
  ;[1 1 1] Casting to doors
  (bind _outactors (Actor|GetAllActorsOfClass "/Game/Blueprints/Doors/BP_DebrisDoor.BP_DebrisDoor_C"))
  (bind _asbp_debris_door (Utilities|Casting|CastToBP_DebrisDoor (Utilities|Array|Get(acopy) _outactors)))
  ;[1 1 1] Adding deleted debris to list
  (Utilities|Array|Add (Variables|/Game/Blueprints/Doors/BP_DebrisDoor.BP_DebrisDoor_C|GetDebris _asbp_debris_door) (Variables|Default|GetDebrisID))
  (Actor|DestroyActor)
  ;[1 1 1] Cheking if list ofe destroyed actors has 3 elements
  (bind _asbp_debris_door_2 (Utilities|Casting|CastToBP_DebrisDoor (Utilities|Array|Get(acopy) _outactors)))
  (if (== (Utilities|Array|Length (Variables|/Game/Blueprints/Doors/BP_DebrisDoor.BP_DebrisDoor_C|GetDebris _asbp_debris_door_2)) 3)
    ;[1 1 1] Setting Doors collision box location (they don't work without it)
    (Transformation|SetRelativeLocation (Variables|/Game/Blueprints/Doors/BP_DebrisDoor.BP_DebrisDoor_C|GetBox _asbp_debris_door_2) "0.000000,0.000000,100.000000" false false)))

(fn ConstructionScript
  (|CallParentFunction))
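; BP_PowerSwitch is an interactable lever that restores power in the command center when pulled.
; BeginInteraction plays the Switch timeline, which rotates the lever's Cube.
; Every timeline update also finds actors by class, turning the first six lights white and stopping their rotation.
; The same update sets IsPowerON on the first monitor and elevator doors actors, repeating this for each light.
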(event EventBeginInteraction
  ;[1 1 1] Pulling switch
  (bind _leverpull (Timeline|Switch Play)
    (:Update
      (Transformation|SetRelativeRotation (Variables|Default|GetCube) (Math|Rotator|Lerp(Rotator) "0.000000,0.000000,30.000000" "0.000000,0.000000,120.000000" _leverpull) false false)
      ;[1 1 1] Casting to BP_CommandCenterLights
      (bind _outactors (Actor|GetAllActorsOfClass "/Game/Blueprints/BPCommandCenterLights.BPCommandCenterLights_C"))
      (for _array_element (Utilities|Array|MakeArray (Utilities|Array|Get(acopy) _outactors) (Utilities|Array|Get(acopy) _outactors 1) (Utilities|Array|Get(acopy) _outactors 2) (Utilities|Array|Get(acopy) _outactors 3) (Utilities|Array|Get(acopy) _outactors 4) (Utilities|Array|Get(acopy) _outactors 5))
        (bind _asbpcommand_center_lights (Utilities|Casting|CastToBPCommandCenterLights _array_element))
        ;[1 1 1] Setting color of lights and deactivating rotation
        (Rendering|Components|Light|SetLightColor (Variables|/Game/Blueprints/BPCommandCenterLights.BPCommandCenterLights_C|GetSpotLight _asbpcommand_center_lights) "(R=1.000000,G=1.000000,B=1.000000,A=1.000000)" true)
        (Components|Activation|Deactivate (Variables|/Game/Blueprints/BPCommandCenterLights.BPCommandCenterLights_C|GetRotatingMovement _asbpcommand_center_lights))
        ;[1 1 1] Casting to BP_CommandCenterMonitor
        (bind _outactors_2 (Actor|GetAllActorsOfClass "/Game/Blueprints/BPCommandCenter_Monitor.BPCommandCenter_Monitor_C"))
        (bind _asbpcommand_center_monitor (Utilities|Casting|CastToBPCommandCenter_Monitor (Utilities|Array|Get(acopy) _outactors_2)))
        (Variables|/Game/Blueprints/BPCommandCenter_Monitor.BPCommandCenter_Monitor_C|SetIsPowerON? _asbpcommand_center_monitor true)
        ;[1 1 1] Casting to BP_CommandCenterElevetorDoors
        (bind _outactors_3 (Actor|GetAllActorsOfClass "/Game/Blueprints/Doors/BP_CommandCenterElevatorDoors.BP_CommandCenterElevatorDoors_C"))
        (bind _asbp_command_center_elevator_doors (Utilities|Casting|CastToBP_CommandCenterElevatorDoors (Utilities|Array|Get(acopy) _outactors_3)))
        (Variables|/Game/Blueprints/Doors/BP_CommandCenterElevatorDoors.BP_CommandCenterElevatorDoors_C|SetIsPowerON? _asbp_command_center_elevator_doors true)))))

(fn ConstructionScript
  (|CallParentFunction))
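; BP_Closet is an interactable closet that opens and spawns a pair of gravity boots.
; On its first BeginInteraction, a DoOnce gate lets it spawn BP_GravityBoots at a hardcoded world location and play the OpenClosetDoor timeline.
; The timeline lerps the relative rotations of two static mesh components in opposite directions, swinging the double doors open.
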(event EventBeginInteraction
  (Utilities|FlowControl|DoOnce false
    (:Completed
      (Game|SpawnActorfromClass "/Game/Blueprints/BP_GravityBoots.BP_GravityBoots_C" (Math|Transform|MakeTransform "-248.000000,-379.000000,5.000000" "0, 0, 0" "1.000000,1.000000,1.000000") "AlwaysSpawn" 0 0)
      (bind _open (Timeline|OpenClosetDoor Play)
        (:Update
          (Transformation|SetRelativeRotation (Variables|Default|GetStaticMesh) (Math|Rotator|Lerp(Rotator) "0.000000,0.000000,0.000000" "0.000000,90.000000,0.000000" _open) false false)
          (Transformation|SetRelativeRotation (Variables|Default|GetStaticMesh1) (Math|Rotator|Lerp(Rotator) "0, 0, 0" "0.000000,-90.000000,0.000000" _open) false false))))))

(fn ConstructionScript
  (|CallParentFunction))
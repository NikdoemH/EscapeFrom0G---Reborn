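; Command center monitor that the player can activate once power is restored, flagging the elevator doors that it is on.
; Tick polls IsPowerON, which is not set in this Blueprint, and uses a DoOnce to switch the screen to a red glow.
; BeginInteraction, when powered, turns the screen green and sets IsMonitorON on the first BP_CommandCenterElevatorDoors found through GetAllActorsOfClass.
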(event EventBeginInteraction
  ;[1 1 1] setting different color of screen
  (if (Variables|Default|GetIsPowerON?)
    (Rendering|Material|SetMaterial (Variables|Default|GetScreen) 0 "/Engine/MapTemplates/Materials/M_Green_Glow.M_Green_Glow")
    ;[1 1 1] Casting to BP_CommandCenterElevatorDoors
    (bind _outactors (Actor|GetAllActorsOfClass "/Game/Blueprints/Doors/BP_CommandCenterElevatorDoors.BP_CommandCenterElevatorDoors_C"))
    (bind _asbp_command_center_elevator_doors (Utilities|Casting|CastToBP_CommandCenterElevatorDoors (Utilities|Array|Get(acopy) _outactors)))
    (Variables|/Game/Blueprints/Doors/BP_CommandCenterElevatorDoors.BP_CommandCenterElevatorDoors_C|SetIsMonitorON? _asbp_command_center_elevator_doors true)))

(event EventTick
  (params (DeltaSeconds :type Float%20%28single-precision%29))
  ;[1 1 1] Checking if player restored power
  (if (Variables|Default|GetIsPowerON?)
    ;[1 1 1] Setting color of screen
    (Utilities|FlowControl|DoOnce false
      (:Completed
        (Rendering|Material|SetMaterial (Variables|Default|GetScreen) 0 "/Engine/MapTemplates/Materials/M_Red_Glow.M_Red_Glow")))))

(fn ConstructionScript
  (|CallParentFunction))
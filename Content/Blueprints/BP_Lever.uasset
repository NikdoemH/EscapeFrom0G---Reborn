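; Interactable lever that toggles the collision box on the left escape pod door.
; On interaction it sets IsLeverPulled, moves the first found BP_EscapePodDoorsLeft's box to a new position, and rotates the handle through a timeline.
; A Delay fired from that timeline's update starts a second timeline about three seconds later, which swings the handle back, clears the flag and lowers the box.
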(event EventBeginInteraction
  ;[1 1 1] hecking if player pulled the lever
  (Variables|Default|SetIsLeverPulled? true)
  ;[1 1 1] Casting to Left side of doors
  (bind _outactors (Actor|GetAllActorsOfClass "/Game/Blueprints/Doors/BP_EscapePodDoorsLeft.BP_EscapePodDoorsLeft_C"))
  (bind _asbp_escape_pod_doors_left (Utilities|Casting|CastToBP_EscapePodDoorsLeft (Utilities|Array|Get(acopy) _outactors)))
  ;[1 1 1] Setting location of collision box
  (Transformation|SetRelativeLocation (Variables|/Game/Blueprints/Doors/BP_EscapePodDoorsLeft.BP_EscapePodDoorsLeft_C|GetBox _asbp_escape_pod_doors_left) "0.000000,250.000000,0.000000" false false)
  ;[1 1 1] Pulling Lever
  (bind _lever_pull (Timeline|Lever PlayFromStart)
    (:Update
      (Transformation|SetRelativeRotation (Variables|Default|GetCube1) (Math|Rotator|Lerp(Rotator) "0.000000,0.000000,30.000000" "0.000000,0.000000,120.000000" _lever_pull) false false)
      (Utilities|FlowControl|Delay 3.0)
      ;[1 1 1] Lever going back in place
      (bind _lever_pull_2 (Timeline|Timeline PlayFromStart)
        (:Update
          (Transformation|SetRelativeRotation (Variables|Default|GetCube1) (Math|Rotator|Lerp(Rotator) "0.000000,0.000000,120.000000" "0.000000,0.000000,30.000000" _lever_pull_2) false false)
          (Variables|Default|SetIsLeverPulled? false)
          ;[1 1 1] Casting to left side of doors
          (bind _outactors_2 (Actor|GetAllActorsOfClass "/Game/Blueprints/Doors/BP_EscapePodDoorsLeft.BP_EscapePodDoorsLeft_C"))
          (bind _asbp_escape_pod_doors_left_2 (Utilities|Casting|CastToBP_EscapePodDoorsLeft (Utilities|Array|Get(acopy) _outactors_2)))
          ;[1 1 1] Setting location of collision box back
          (Transformation|SetRelativeLocation (Variables|/Game/Blueprints/Doors/BP_EscapePodDoorsLeft.BP_EscapePodDoorsLeft_C|GetBox _asbp_escape_pod_doors_left_2) "0.000000,250.000000,-200.000000" false false))))))

(fn ConstructionScript
  (|CallParentFunction))